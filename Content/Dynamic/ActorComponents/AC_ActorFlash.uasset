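; AC_ActorFlash is an actor component that swaps its owner's static mesh materials to show flash and death states.
; On BeginPlay it caches the first-slot material of every static mesh component on the owner in a map keyed by component.
; StartFlash and StartDeath apply the flash or death material to slot 0 of those meshes, and EndFlash restores the cached originals.
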(event `self.ReceiveBeginPlay`
  (for _array_element (`Actor.K2_GetComponentsByClass` (`self.GetOwner`) "/Script/Engine.StaticMeshComponent")
    (`BlueprintMapLibrary.Map_Add` (`self.InitialStaticMeshMaterials`) _array_element (`PrimitiveComponent.GetMaterial` _array_element 0))))

(fn `EndFlash`
  (bind _initialstaticmeshmaterials (`self.InitialStaticMeshMaterials`))
  (bind _keys (`BlueprintMapLibrary.Map_Keys` _initialstaticmeshmaterials))
  (for _array_element _keys
    (bind (_value _returnvalue) (`BlueprintMapLibrary.Map_Find` _initialstaticmeshmaterials _array_element))
    (if _returnvalue
      (`PrimitiveComponent.SetMaterial` _array_element 0 _value))))

(fn `StartDeath`
  (bind _keys (`BlueprintMapLibrary.Map_Keys` (`self.InitialStaticMeshMaterials`)))
  (for _array_element _keys
    (`PrimitiveComponent.SetMaterial` _array_element 0 (`self.DeathMaterial`))))

(fn `StartFlash`
  (bind _keys (`BlueprintMapLibrary.Map_Keys` (`self.InitialStaticMeshMaterials`)))
  (for _array_element _keys
    (`PrimitiveComponent.SetMaterial` _array_element 0 (`self.FlashMaterial`))))