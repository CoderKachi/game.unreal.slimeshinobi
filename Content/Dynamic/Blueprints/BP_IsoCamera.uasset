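; BP_IsoCamera is an orthographic follow camera that makes itself the player's view target on begin play.
; With AutoFindPlayer set, it targets the controlled pawn, registers with BP_TopDownController and updates its movement axes.
; Each tick it lerps toward GetTargetTransform and eases ortho width toward FollowDistance, both using FollowSpeed as alpha.
; Setter functions change the target, speed and distance.
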(event `self.ReceiveBeginPlay`
  (bind _returnvalue (`GameplayStatics.GetPlayerController` 0))
  (`PlayerController.SetViewTargetWithBlend` _returnvalue self 0.0 "VTBlend_Linear" 0.0 false)
  (if (`self.AutoFindPlayer`)
    (set `self.TargetActor` (`Controller.K2_GetPawn` _returnvalue))
    (bind _asbp_top_down_controller (cast `/Game/Dynamic/Blueprints/BP_TopDownController` _returnvalue))
    (set `/Game/Dynamic/Blueprints/BP_TopDownController.CurrentCamera` self _asbp_top_down_controller)
    (`/Game/Dynamic/Blueprints/BP_TopDownController.UpdateMovementAxis` _asbp_top_down_controller)))

(event `self.ReceiveTick`
  (params (DeltaSeconds :type "Float (single-precision)"))
  (`self.LerpOrthoWidth`)
  (`self.K2_SetActorTransform` self (`KismetMathLibrary.TLerp` (`self.GetTransform` self) (`self.GetTargetTransform`) (`self.FollowSpeed`)) false false))

(fn `SetDistance`
  (params (NewFollowDistance :type "Float (double-precision)"))
  (set `self.FollowDistance` NewFollowDistance))

(fn `SetSpeed`
  (params (NewFollowSpeed :type "Float (double-precision)"))
  (set `self.FollowSpeed` NewFollowSpeed))

(fn `SetTarget`
  (params (NewTargetActor :type "Actor Object Reference"))
  (`/Engine/EditorBlueprintResources/StandardMacros.IsValid` NewTargetActor
    (:`Is Valid`
      (set `self.TargetActor` NewTargetActor))
    (:`Is Not Valid`
      (`KismetSystemLibrary.PrintString` "Failed to set Target Actor"))))

(fn `UserConstructionScript`)