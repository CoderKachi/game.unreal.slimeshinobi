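; Enemy character that splits in two whenever it takes damage, with no other active logic in this graph.
; On damage it shrinks its capsule, spawns a copy through ActorSplitter and copies max and current health to it.
; Both are offset by the capsule diameter and launched with random upward impulses, with subtraction and negation meant to separate them, though the random values are rolled inline rather than stored.
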(event `self.HealthComponent.OnDamageTaken`
  (bind _healthcomponent (`self.HealthComponent`))
  (bind _capsulecomponent (`self.CapsuleComponent`))
  (bind _returnvalue (* (`KismetMathLibrary.MakeVector` (`KismetMathLibrary.RandomFloatInRange` -10.0 10.0) (`KismetMathLibrary.RandomFloatInRange` -10.0 10.0) (`KismetMathLibrary.RandomFloatInRange` 2.5 10.0)) (`KismetMathLibrary.RandomFloatInRange` 10.0 100.0)))
  (bind (_returnvalue_x _returnvalue_y) (`KismetMathLibrary.BreakVector2D` (`KismetMathLibrary.Negated2D` (`KismetMathLibrary.MakeVector2D` (.x _returnvalue) (.y _returnvalue)))))
  (`SceneComponent.SetRelativeScale3D` _capsulecomponent (* (`SceneComponent.RelativeScale3D` _capsulecomponent) 0.8))
  (bind _clone (`/Game/Dynamic/Blueprints/AC_ActorSplitter.SplitSelf` (`self.ActorSplitter`)))
  (bind _returnvalue_2 (`self.GetComponentByClass` _clone "/Game/Dynamic/Blueprints/Pi/ActorComponents/HealthComponent.HealthComponent_C"))
  (set `/Game/Dynamic/Blueprints/Pi/ActorComponents/HealthComponent.HealthMax` (`/Game/Dynamic/Blueprints/Pi/ActorComponents/HealthComponent.HealthMax` _healthcomponent) _returnvalue_2)
  (set `/Game/Dynamic/Blueprints/Pi/ActorComponents/HealthComponent.HealthCurrent` (`/Game/Dynamic/Blueprints/Pi/ActorComponents/HealthComponent.HealthCurrent` _healthcomponent) _returnvalue_2)
  (`/Game/Dynamic/Blueprints/Pi/ActorComponents/HealthComponent.UpdateHealth` _returnvalue_2)
  (bind (_returnvalue_x_2 _returnvalue_y_2) (`KismetMathLibrary.BreakVector2D` (* (`KismetMathLibrary.Normal2D` (`KismetMathLibrary.MakeVector2D` (`KismetMathLibrary.RandomFloatInRange` -1.0 1.0) (`KismetMathLibrary.RandomFloatInRange` -1.0 1.0))) (* (`CapsuleComponent.GetScaledCapsuleSize` (`self.GetComponentByClass` _clone "/Script/Engine.CapsuleComponent")) 2.0))))
  (`self.K2_SetActorLocation` _clone (+ (`self.K2_GetActorLocation` _clone) (`KismetMathLibrary.MakeVector` _returnvalue_x_2 _returnvalue_y_2)) false false)
  (`self.K2_SetActorLocation` (- (`self.K2_GetActorLocation`) (`KismetMathLibrary.MakeVector` _returnvalue_x_2 _returnvalue_y_2)))
  (`CharacterMovementComponent.AddImpulse` (`self.GetComponentByClass` _clone "/Script/Engine.CharacterMovementComponent") _returnvalue true)
  (`CharacterMovementComponent.AddImpulse` (`self.CharacterMovement`) (`KismetMathLibrary.MakeVector` _returnvalue_x _returnvalue_y (.z _returnvalue)) true))

(fn `UserConstructionScript`)