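; Isometric follow camera actor that becomes player 0's view target on BeginPlay and tracks that player's controlled pawn.
; Tick eases it toward a point FollowDistance behind the target along TargetRotation, with FollowDistance also driving ortho width.
; Smoothing lerps by FollowSpeed each frame, without delta-time scaling.
; Setters change target, speed and distance at runtime; an older top-down follow branch is left unconnected.
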(event `self.ReceiveBeginPlay`
  (bind _returnvalue (`GameplayStatics.GetPlayerController` 0))
  (`PlayerController.SetViewTargetWithBlend` _returnvalue self 0.0 "VTBlend_Linear" 0.0 false)
  (set `self.TargetActor` (`Controller.K2_GetPawn` _returnvalue)))

(event `self.ReceiveTick`
  (params (DeltaSeconds :type "Float (single-precision)"))
  (bind _targetactor (`self.TargetActor`))
  (bind _targetrotation (`self.TargetRotation`))
  (bind _cameracomponent (`self.CameraComponent`))
  (`/Engine/EditorBlueprintResources/StandardMacros.IsValid` _targetactor
    (:`Is Valid`
      (`CameraComponent.SetOrthoWidth` _cameracomponent (`KismetMathLibrary.Lerp` (`CameraComponent.OrthoWidth` _cameracomponent) (`self.FollowDistance`) (`self.FollowSpeed`)))
      (`self.K2_SetActorTransform` (`KismetMathLibrary.TLerp` (`self.GetTransform` self) (`KismetMathLibrary.MakeTransform` (+ (`self.K2_GetActorLocation` _targetactor) (* (`KismetMathLibrary.GetForwardVector` _targetrotation) (* (`self.FollowDistance`) -1.0))) _targetrotation) (`self.FollowSpeed`))))))

(fn `SetDistance`
  (params (NewFollowDistance :type "Float (double-precision)"))
  (set `self.FollowDistance` NewFollowDistance))

(fn `SetSpeed`
  (params (NewFollowSpeed :type "Float (double-precision)"))
  (set `self.FollowSpeed` NewFollowSpeed))

(fn `SetTarget`
  (params (NewTargetActor :type "Actor Object Reference"))
  (`/Engine/EditorBlueprintResources/StandardMacros.IsValid` NewTargetActor
    (:`Is Valid`
      (set `self.TargetActor` NewTargetActor))
    (:`Is Not Valid`
      (`KismetSystemLibrary.PrintString` "Failed to set Target Actor"))))

(fn `UserConstructionScript`)