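; BP_SlimeSpawner is a tagged spawn point that spawns queued slime classes at its own transform.
; QueueSlime adds a class and calls SpawnSlime right away only if no BP_Enemy overlaps its sphere.
; SpawnSlime spawns and removes the head entry, then sets a timer by function name to call itself after SpawnDelay.
; The queue stores only classes, so initial health is not kept per entry for timed spawns.
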(event `self.ReceiveBeginPlay`)

(fn `QueueSlime`
  (params (SlimeClass :type "/Game/Dynamic/Blueprints/BP_Enemy Class Reference (by ref)") (InitialHealth :type Integer))
  (`KismetArrayLibrary.Array_Add` (`self.Queue`) SlimeClass)
  (if (not (`KismetArrayLibrary.Array_IsValidIndex` (`PrimitiveComponent.GetOverlappingActors` (`self.Sphere`) "/Game/Dynamic/Blueprints/BP_Enemy.BP_Enemy_C")))
    (`self.SpawnSlime` InitialHealth)))

(fn `SpawnSlime`
  (params (IntitalHealth :type Integer))
  (returns (Success :type Boolean))
  (bind _queue (`self.Queue`))
  (if (`KismetArrayLibrary.Array_IsValidIndex` _queue)
    (`|SpawnActorFromClass` (`|GetArrayItem` _queue) (`self.GetTransform`) "AlwaysSpawn" "MultiplyWithRoot" null IntitalHealth null)
    (`KismetArrayLibrary.Array_Remove` _queue)
    (`KismetSystemLibrary.K2_SetTimer` null "SpawnSlime" (`self.SpawnDelay`))
    (return true)
    (else
      (return false))))

(fn `UserConstructionScript`
  (`KismetArrayLibrary.Array_Add` (`self.Tags`) (`self.SpawnerTag`)))