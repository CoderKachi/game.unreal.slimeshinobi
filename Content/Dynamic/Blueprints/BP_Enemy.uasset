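; BP_Enemy is a slime enemy that splits into smaller slimes when damaged, scaling its size by max health.
; Non-stun damage spawns 2^damage clones via ActorSplitter, launches them in a ring and destroys the original.
; Zero-health deaths report to BP_TopDownGameMode, while stun hits trigger ActorFlash effects.
; Attack shows a timed area warning, then capsule-traces to damage non-slime pawns, with timing based on health and speed.
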(event `UpdateSize`
  (`SceneComponent.SetRelativeScale3D` (`self.CapsuleComponent`) (* (`self.Initial Relative Scale 3D`) (`KismetMathLibrary.MultiplyMultiply_FloatFloat` 0.8 (- 3.0 (`KismetMathLibrary.Conv_IntToDouble` (`/Game/Dynamic/ActorComponents/HealthComponent.HealthMax` (`self.HealthComponent`))))))))

(event `self.ReceiveBeginPlay`
  (bind _healthcomponent (`self.HealthComponent`))
  (bind _inithealth (`self.InitHealth`))
  (bind _output_get (set `/Game/Dynamic/ActorComponents/HealthComponent.HealthMax` (`KismetMathLibrary.SelectInt` _inithealth (`/Game/Dynamic/ActorComponents/HealthComponent.HealthMax` _healthcomponent) (!= _inithealth -1)) _healthcomponent))
  (set `/Game/Dynamic/ActorComponents/HealthComponent.HealthCurrent` _output_get _healthcomponent)
  (`/Game/Dynamic/ActorComponents/HealthComponent.UpdateHealth` _healthcomponent)
  (`self.UpdateSize`)
  (set `CharacterMovementComponent.MaxWalkSpeed` (* 300.0 (`self.SpeedMultiplier`)) (`self.CharacterMovement`)))

(event `self.HealthComponent.OnDamageTaken`
  (bind _actorflash (`self.ActorFlash`))
  (bind _clones (`self.Clones`))
  (bind (_lastdamageinfo_amount _lastdamageinfo_damagetype _lastdamageinfo_damageresponse _lastdamageinfo_direction) (break `/Game/Dynamic/DataStructures/S_DamageInfo` (`/Game/Dynamic/ActorComponents/HealthComponent.LastDamageInfo` (`self.HealthComponent`))))
  (bind (_lastdamageinfo_amount_2 _lastdamageinfo_damagetype_2 _lastdamageinfo_damageresponse_2) (break `/Game/Dynamic/DataStructures/S_DamageInfo` (`/Game/Dynamic/ActorComponents/HealthComponent.LastDamageInfo` (`self.HealthComponent`))))
  (switch `/Game/Dynamic/DataStructures/E_DamageResponse` _lastdamageinfo_damageresponse_2
    (:`NewEnumerator0`
      (bind (_healthcomponent _returnvalue) (`self.CalculateHealth`)
        (:`then`
          (`/Game/Dynamic/ActorComponents/HealthComponent.UpdateHealth` _healthcomponent)
          (`/Game/Dynamic/ActorComponents/AC_ActorFlash.EndFlash` (`self.ActorFlash`))
          (`KismetArrayLibrary.Array_Clear` _clones)
          (set `self.SpawnVector` (* (`KismetMathLibrary.GetRotated2D` _lastdamageinfo_direction 90.0) (* (`CapsuleComponent.GetScaledCapsuleSize` (`self.CapsuleComponent`)) 3.0)))
          (for _ (range 1 (+ (`KismetMathLibrary.FTrunc` _returnvalue) 1))
            (`self.CloneSlimes` _clones))
          (for (_array_element _array_index) _clones
            (`self.InitialiseSlimePositions` _array_element _array_index))
          (set `self.Height` (`KismetMathLibrary.RandomFloatInRange` 2.5 10.0))
          (set `self.Magnitude` (`KismetMathLibrary.RandomFloatInRange` 30.0 50.0))
          (for (_array_element_2 _array_index_2) (`self.Clones`)
            (`self.LaunchSlimes` _array_element_2 _array_index_2
              (:`Completed`
                (bind _asbp_enemy (cast `/Game/Dynamic/Blueprints/BP_Enemy` _array_element_2))
                (`self.UpdateSize` _asbp_enemy))))
          (`/Game/Dynamic/ActorComponents/HealthComponent.OnDeath` (`self.HealthComponent`)))))
    (:`NewEnumerator1`
      (if (> (`/Game/Dynamic/ActorComponents/HealthComponent.HealthCurrent` (`self.HealthComponent`)) 1)
        (`/Game/Dynamic/ActorComponents/AC_ActorFlash.StartFlash` _actorflash)
        (`KismetSystemLibrary.RetriggerableDelay` 1.0)
        (`/Game/Dynamic/ActorComponents/AC_ActorFlash.EndFlash` _actorflash)
        (else
          (`/Game/Dynamic/ActorComponents/AC_ActorFlash.StartDeath` _actorflash))))))

(event `self.HealthComponent.OnDeath`
  (if (<= (`/Game/Dynamic/ActorComponents/HealthComponent.HealthCurrent` (`self.HealthComponent`)) 0)
    (bind _asbp_top_down_game_mode (cast `/Game/Dynamic/Blueprints/BP_TopDownGameMode` (`GameplayStatics.GetGameMode`)))
    (`/Game/Dynamic/Blueprints/BP_TopDownGameMode.OnSlimeDefeated` _asbp_top_down_game_mode (`KismetMathLibrary.FTrunc` (`KismetMathLibrary.MultiplyMultiply_FloatFloat` 2.0 (`KismetMathLibrary.Conv_IntToDouble` (- (`self.DamageTaken`) 1))))))
  (`self.K2_DestroyActor`))

(event `Attack`
  (bind _returnvalue (`self.K2_GetActorLocation`))
  (bind _relativescale3d_x (`KismetMathLibrary.BreakVector` (`SceneComponent.RelativeScale3D` (`self.CapsuleComponent`))))
  (bind _returnvalue_2 (/ (+ (* (`/Game/Dynamic/ActorComponents/HealthComponent.HealthMax` (`self.HealthComponent`)) 0.25) 0.75) (`self.SpeedMultiplier`)))
  (`self.CreateAttackWarning` 0.0 (* _relativescale3d_x (`self.AttackRadiusMultiplier`)) _returnvalue_2
    (:`Completed`
      (`KismetSystemLibrary.Delay` _returnvalue_2)
      (bind _outhits (`KismetSystemLibrary.CapsuleTraceMultiForObjects` :`Start` _returnvalue :`End` _returnvalue :`Radius` (* (`CapsuleComponent.GetScaledCapsuleSize` (`self.CapsuleComponent`)) (`self.AttackRadiusMultiplier`)) :`ObjectTypes` (`|MakeArray` "ObjectTypeQuery3" :!type "EObjectTypeQuery Enum") :`DrawTime` 20.0))
      (for _array_element _outhits
        (bind _returnvalue_3 (`self.GetComponentByClass` (`.HitActor` (`GameplayStatics.BreakHitResult` _array_element)) "/Game/Dynamic/ActorComponents/HealthComponent.HealthComponent_C"))
        (`/Engine/EditorBlueprintResources/StandardMacros.IsValid` _returnvalue_3
          (:`Is Valid`
            (if (not (`/Game/Dynamic/ActorComponents/HealthComponent.IsSlime` _returnvalue_3))
              (`/Game/Dynamic/ActorComponents/HealthComponent.TakeDamage` _returnvalue_3 (make `/Game/Dynamic/DataStructures/S_DamageInfo` 1))))))
      (`self.OnAttackEnd`))))

(fn `UserConstructionScript`
  (locals (NewLocalVar :type Boolean)))