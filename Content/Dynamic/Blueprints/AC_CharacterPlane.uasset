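; Actor component that computes the rotation from its owner toward the mouse cursor on a plane through the owner.
; FindRotationToMouse deprojects the cursor from player controller 0 and intersects that ray with a plane at the owner's location, using the controller's up vector as normal.
; It returns the look-at rotation to the hit point and draws a blue debug line there.
; The event graph holds no active logic.
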(fn `FindRotationToMouse`
  (returns (LookAtRotation :type "Rotator Structure"))
  (bind _returnvalue (`GameplayStatics.GetPlayerController` 0))
  (bind (_worldlocation _worlddirection) (`PlayerController.DeprojectMousePositionToWorld` _returnvalue))
  (bind _returnvalue_2 (`Actor.GetActorUpVector` _returnvalue))
  (bind _returnvalue_3 (`Actor.K2_GetActorLocation` (`self.GetOwner`)))
  (bind (_t _intersection) (`KismetMathLibrary.LinePlaneIntersection_OriginNormal` _worldlocation (+ _worldlocation (* _worlddirection 9999.0)) _returnvalue_3 _returnvalue_2))
  (`KismetSystemLibrary.DrawDebugLine` _intersection (+ _intersection (* _returnvalue_2 100.0)) (struct :`G` 0.255585 :`B` 1.0 :`A` 1.0))
  (return (`KismetMathLibrary.FindLookAtRotation` _returnvalue_3 _intersection)))